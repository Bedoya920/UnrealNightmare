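; Zombie enemy that wanders to random reachable points and chases pawns it sees, returning to wandering after losing sight.
; Movement uses AIMoveTo, with PawnSensing triggering the faster chase and a retriggerable delay ending it.
; Reaching the target starts a gated attack montage that halts movement and applies sphere-overlap damage on its notify.
; Incoming damage feeds BPCStats and plays a hit reaction; death enables ragdoll and ignores Visibility and Pawn collision.
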(event `self.ReceiveBeginPlay`
  ; Begin play
  (`self.Wandering`))

(event `Wandering`
  ; Zombie Wandering around
  (set `CharacterMovementComponent.MaxWalkSpeed` 80.0 (`self.CharacterMovement`))
  (`|AIMoveTo` self (`NavigationSystemV1.K2_GetRandomReachablePointInRadius` (`SceneComponent.K2_GetComponentLocation` (`self.Mesh`)) 1000.0 null null) null
    (:`OnSuccess`
      (`KismetSystemLibrary.Delay` (`KismetMathLibrary.RandomFloatInRange` 1.0 3.0))
      (`self.Wandering`))))

(event `self.PawnSensing.OnSeePawn`
  (params (Pawn :type "Pawn Object Reference"))
  ; Zombie chase player
  (`|ExecutionSequence`
    (:`then_0`
      (set `CharacterMovementComponent.MaxWalkSpeed` 400.0 (`self.CharacterMovement`))
      (`|AIMoveTo` self (0.0 0.0 0.0) Pawn
        (:`OnSuccess`
          (`self.Zombie Attack`))))
    (:`then_1`
      ; Zombie stop chasing player if out of sight
      (`KismetSystemLibrary.RetriggerableDelay` 3.0)
      (`self.Wandering`))))

(event `Zombie Attack`
  ; Zombie atack
  (if (not (`self.IsDead`))
    (`/Engine/EditorBlueprintResources/StandardMacros.DoOnce` false :!label _label
      (:`Completed`
        (`CharacterMovementComponent.DisableMovement` (`self.CharacterMovement`))
        (`|PlayMontage` (`self.Mesh`) "/Game/TPShooter/Animations/Zombie/AM_Zombie_Attack_Montage.AM_Zombie_Attack_Montage"
          (:`then`
            (`GameplayStatics.PlaySound2D` null 1.0 1.0 0.0 null null))
          (:`OnCompleted`
            (`CharacterMovementComponent.SetMovementMode` (`self.CharacterMovement`) "MOVE_Walking" 0 :!label _label_2)
            (goto _label :!via `Reset`))
          (:`OnInterrupted`
            (`KismetSystemLibrary.Delay` 0.5)
            (goto _label_2))
          (:`OnNotifyBegin`
            (`self.Zombie Attack Damage`)))))))

(event `Zombie Attack Damage`
  ; Zombie Deal Damage
  (bind _outactors (`KismetSystemLibrary.SphereOverlapActors` (`SceneComponent.K2_GetComponentLocation` (`self.Zombie Damage`)) (`self.ZombieRange`) (`|MakeArray` "ObjectTypeQuery3" :!type "EObjectTypeQuery Enum") "/Script/Engine.Actor" (`|MakeArray` self :!type "Actor Object Reference")))
  (for _array_element _outactors
    (`GameplayStatics.ApplyDamage` _array_element (`self.Base Damage`) (`self.GetController`) self "/Script/Engine.DamageType")))

(event `self.ReceiveAnyDamage`
  (params (Damage :type "Float (single-precision)") (DamageType :type "DamageType Object Reference") (InstigatedBy :type "Controller Object Reference") (DamageCauser :type "Actor Object Reference"))
  (bind _mesh (`self.Mesh`))
  ; Zombie gets Damage
  (bind _dead (`/Game/TPShooter/Blueprints/Stats/BPC_Stats.Decrease HP` (`self.BPC_Stats`) Damage))
  (`|PlayMontage` (`self.Mesh`) "/Game/TPShooter/Animations/Zombie/AM_Zombie_Reaction_Hit_Montage.AM_Zombie_Reaction_Hit_Montage"
    (:`then`
      (if _dead
        (`PrimitiveComponent.SetSimulatePhysics` (`self.Mesh`) true)
        (`PrimitiveComponent.SetCollisionResponseToChannel` _mesh "ECC_Visibility" "ECR_Ignore")
        (`PrimitiveComponent.SetCollisionResponseToChannel` (`self.CapsuleComponent`) "ECC_Visibility" "ECR_Ignore")
        (`PrimitiveComponent.SetCollisionResponseToChannel` _mesh "ECC_Pawn" "ECR_Ignore")
        (`PrimitiveComponent.SetCollisionResponseToChannel` (`self.CapsuleComponent`) "ECC_Pawn" "ECR_Ignore")
        (set `self.IsDead` true)))))

(fn `UserConstructionScript`)