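; Actor component that tracks hit points and stamina for its owner in the third-person shooter.
; BeginPlay fills current HP and stamina from their maximum values.
; Decrease functions subtract an amount and return true once the value reaches zero or below, without clamping at zero.
; Increase functions add an amount and cap it at the maximum.
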(event `self.ReceiveBeginPlay`
  (set `self.CurrentHP` (`self.HitPoints`))
  (set `self.CurrentStamina` (`self.Stamina`)))

(fn `Decrease HP`
  (params (Damage :type "Float (double-precision)"))
  (returns (Dead :type Boolean))
  (set `self.CurrentHP` (- (`self.CurrentHP`) Damage))
  (if (<= (`self.CurrentHP`) 0.0)
    (return true)
    (else
      (return false))))

(fn `Decrease Stamina`
  (params (`Decrease Stamina` :type "Float (double-precision)"))
  (returns (Tired :type Boolean))
  (set `self.CurrentStamina` (- (`self.CurrentStamina`) `Decrease Stamina`))
  (if (<= (`self.CurrentStamina`) 0.0)
    (return true)
    (else
      (return false))))

(fn `Increase HP`
  (params (Healing :type "Float (double-precision)"))
  (set `self.CurrentHP` (+ (`self.CurrentHP`) Healing))
  (if (> (`self.CurrentHP`) (`self.HitPoints`))
    (set `self.CurrentHP` (`self.HitPoints`))))

(fn `Increase Stamina`
  (params (`Increase Stamina` :type "Float (double-precision)"))
  (set `self.CurrentStamina` (+ (`self.CurrentStamina`) `Increase Stamina`))
  (if (> (`self.CurrentStamina`) (`self.Stamina`))
    (set `self.CurrentStamina` (`self.Stamina`))))