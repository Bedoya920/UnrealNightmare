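; BP_Simple_Door is a hinged door that swings open away from or toward a given location and closes again on the next OpenDoor call.
; A dot product between the actor's forward vector and the direction to that location picks a 90-degree swing in either direction.
; A FlipFlop alternates playing and reversing the TLDoor timeline, which lerps the Door component's relative yaw, and calls during playback are ignored.
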(event `Open Door`
  (params (Location :type "Vector Structure"))
  (if (not (`TimelineComponent.IsPlaying` (`self.TL Door`)))
    (`/Engine/EditorBlueprintResources/StandardMacros.FlipFlop`
      (:`A`
        (set `self.DoorRotation` (`KismetMathLibrary.SelectFloat` -90.0 90.0 (>= (`KismetMathLibrary.Dot_VectorVector` (`KismetMathLibrary.GetDirectionUnitVector` (`self.K2_GetActorLocation`) Location) (`self.GetActorForwardVector`)) 0.0)))
        (bind (_direction _doorangle) (`Timeline|TL Door` :!via `PlayFromStart` :!label _label)
          (:`Update`
            (`SceneComponent.K2_SetRelativeRotation` (`self.Door`) (`KismetMathLibrary.MakeRotator` 0.0 0.0 (`KismetMathLibrary.Lerp` 0.0 (`self.DoorRotation`) _doorangle)) false false))))
      (:`B`
        (goto _label :!via `Reverse`)))))

(fn `UserConstructionScript`)